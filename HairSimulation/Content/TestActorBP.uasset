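; TestActorBP is a test actor that slides along its local X axis while IsMove is true.
; Each Tick sets Dir to 1 and offsets DefaultSceneRoot by a fixed, frame-rate-dependent step without sweep.
; World X bound checks that would flip Dir for back-and-forth motion between 0 and 100 are disconnected, so it only moves forward.
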(event EventBeginPlay)

(event Collision|EventActorBeginOverlap
  (params (OtherActor :type Actor%20Object%20Reference)))

(event EventTick
  (params (DeltaSeconds :type Float%20%28single-precision%29))
  (if (Variables|Default|GetIsMove)
    (Variables|Default|Setdir 1.0)
    (Class|SceneComponent|AddLocalTransform (Variables|Default|GetDefaultSceneRoot) (Math|Transform|MakeTransform (Math|Vector|MakeVector (* (Variables|Default|Getdir) 1.0) 0.0 0.0)) false false)))

(fn ConstructionScript)